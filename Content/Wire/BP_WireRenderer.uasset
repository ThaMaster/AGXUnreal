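; Deprecated Blueprint that draws an AGX Wire with pooled spline mesh components and prints a deprecation warning on construction.
; It finds the wire from a set reference, attach ancestors or the owning actor, optionally by name, re-resolving via soft reference.
; Each tick it reads render node locations and places meshes either one per segment or at even intervals along a spline, hiding extras.
; Debug flags draw points, tangents and segments.
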(event `self.ReceiveBeginPlay`
  ;[1 1 1] Begin Play.
)

(event `self.ReceiveTick`
  (params (DeltaSeconds :type "Float (single-precision)"))
  ;[1 1 1] Tick
  (bind _have_wire (`self.Update Wire Reference` false))
  (if _have_wire
    (`self.Render`)
    (else
      (`self.Hide All Spline Meshes`))))

(fn `Create Spline Mesh`
  (bind _returnvalue (`AddComponent|NODE_AddSplineMeshComponent-2` :`bManualAttachment` true)) ; TODO: Add support for Material to this execution chain.
  (`SceneComponent.SetMobility` _returnvalue "Movable")
  (`PrimitiveComponent.SetMaterial` _returnvalue 0 (`self.Material`))
  (`StaticMeshComponent.SetStaticMesh` _returnvalue (`self.Mesh`))
  (`SplineMeshComponent.SetForwardAxis` _returnvalue (`self.Mesh Forward`) false)
  (`SplineMeshComponent.SetSplineUpDir` _returnvalue (`KismetMathLibrary.Vector_Forward`) false) ; May need some logic here.
  (`KismetArrayLibrary.Array_Add` (`self.Spline Meshes`) _returnvalue))

(fn `Debug Draw Spline Mesh`
  (params (Start :type "Vector Structure") (End :type "Vector Structure"))
  (if (`self.Debug Render Spline Mesh Points`)
    (`KismetSystemLibrary.DrawDebugCylinder` Start End (* (`AGX_WireComponent.Radius` (`self.Wire`)) 2.0) 8 (struct :`G` 0.14412 :`B` 0.46875 :`A` 1.0) 0.0 (`self.Debug Thickness`))))

(fn `Debug Draw Tangents`
  (bind _spline (`self.Spline`))
  (for _index (range (+ (`SplineComponent.GetNumberOfSplinePoints` _spline) 1))
    (bind _returnvalue (`SplineComponent.GetLocationAtSplinePoint` _spline _index "World"))
    (`KismetSystemLibrary.DrawDebugLine` _returnvalue (+ _returnvalue (`SplineComponent.GetLeaveTangentAtSplinePoint` _spline _index "World")) (struct :`R` 0.760417 :`A` 1.0) 0.0 (`self.Debug Thickness`))
    (`KismetSystemLibrary.DrawDebugLine` _returnvalue (- _returnvalue (`SplineComponent.GetArriveTangentAtSplinePoint` _spline _index "World")) (struct :`G` 0.097717 :`B` 0.71875 :`A` 1.0) 0.0 (`self.Debug Thickness`))))

(fn `Debug Draw Wire`
  (for _array_element (`self.Points`)
    (`KismetSystemLibrary.DrawDebugSphere` _array_element (* (`AGX_WireComponent.Radius` (`self.Wire`)) 2.0) 5 (struct :`R` 0.703125 :`G` 0.354109 :`A` 1.0) 0.0 (`self.Debug Thickness`))))

(fn `Distance Scale Tangents`
  (bind _spline (`self.Spline`))
  (bind _spline_2 (`self.Spline`))
  (`SplineComponent.UpdateSpline` _spline_2)
  (for _index (range 1 (`SplineComponent.GetNumberOfSplinePoints` _spline_2))
    (bind _returnvalue (`SplineComponent.GetLocationAtSplinePoint` _spline _index "World"))
    (`SplineComponent.SetTangentsAtSplinePoint` _spline _index (* (`KismetMathLibrary.Normal` (`SplineComponent.GetArriveTangentAtSplinePoint` _spline _index "World")) (`KismetMathLibrary.VSize` (- (`SplineComponent.GetLocationAtSplinePoint` _spline (- _index 1) "World") _returnvalue))) (* (`KismetMathLibrary.Normal` (`SplineComponent.GetLeaveTangentAtSplinePoint` _spline _index "World")) (`KismetMathLibrary.VSize` (- _returnvalue (`SplineComponent.GetLocationAtSplinePoint` _spline (+ _index 1) "World")))) "World" false)))

(fn `Find Wire`
  (params (`Suppress Warnings` :type Boolean))
  (bind _defaultsceneroot (`self.DefaultSceneRoot`))
  (bind _wire (`self.Wire`))
  (bind _returnvalue (`KismetSystemLibrary.GetDisplayName` self))
  ;[1 1 1] Check if user provided a Wire. That overrules everything else.
  (`/Engine/EditorBlueprintResources/StandardMacros.IsValid` _wire
    (:`Is Valid`
      (set `self.WireSoftRef` (`|ConvertAsset` _wire)))
    (:`Is Not Valid`
      ;[1 1 1] We must have a Default Scene Root in order to have a context to search in.
      (`/Engine/EditorBlueprintResources/StandardMacros.IsValid` _defaultsceneroot
        (:`Is Valid`
          (`/Engine/EditorBlueprintResources/StandardMacros.IsValid` (`SceneComponent.GetAttachParent` _defaultsceneroot)
            (:`Is Valid`
              ;[1 1 1] Look for a Wire in our attachment ancestor chain.
              (bind _wire_2 (`self.Find Wire In Attach Ancestor Chain`))
              (`/Engine/EditorBlueprintResources/StandardMacros.IsValid` _wire_2
                (:`Is Valid`
                  (bind _output_get (set `self.Wire` _wire_2))
                  (set `self.WireSoftRef` (`|ConvertAsset` _output_get)))
                (:`Is Not Valid`
                  ;[1 1 1] Look for a Wire within the entire Actor that we are attached to.
                  (bind _wire_3 (`self.Find Wire In Actor` (`ActorComponent.GetOwner` (`SceneComponent.GetAttachParent` (`self.DefaultSceneRoot`)))))
                  (`/Engine/EditorBlueprintResources/StandardMacros.IsValid` _wire_3
                    (:`Is Valid`
                      (bind _output_get_2 (set `self.Wire` _wire_3))
                      (set `self.WireSoftRef` (`|ConvertAsset` _output_get_2)))
                    (:`Is Not Valid`
                      ;[1 1 1] Fail, did not find a Wire to render.
                      (if (not `Suppress Warnings`)
                        (`KismetSystemLibrary.PrintString` (`KismetStringLibrary.Concat_StrStr` "Wire renderer " (`KismetSystemLibrary.GetObjectName` self) " did not find a wire to render."))))))))
            (:`Is Not Valid`
              (if (not `Suppress Warnings`)
                (`KismetSystemLibrary.PrintString` (`KismetStringLibrary.Concat_StrStr` "Wire Renderer " _returnvalue " does not have an Attach Parent. Cannot find Wire to render."))))))
        (:`Is Not Valid`
          (if (not `Suppress Warnings`)
            (`KismetSystemLibrary.PrintString` (`KismetStringLibrary.Concat_StrStr` "Wire Renderer " _returnvalue " does not have a Default Scene Root. Cannot find Wire to render."))))))))

(fn `Find Wire In Actor`
  (params (Actor :type "Actor Object Reference"))
  (returns (Wire :type "AGX_WireComponent Object Reference"))
  (`/Engine/EditorBlueprintResources/StandardMacros.IsValid` Actor
    (:`Is Valid`
      (for _array_element (`self.K2_GetComponentsByClass` Actor "/Script/AGXUnreal.AGX_WireComponent")
        (bind (_is_wanted_wire _wanted_wire) (`self.Is Wanted Wire` _array_element)
          (:`Yes`
            (return _wanted_wire)))))
    (:`Is Not Valid`
      _))
  (return null))

(fn `Find Wire In Attach Ancestor Chain`
  (returns (Wire :type "AGX_WireComponent Object Reference"))
  (locals (Ancestor :type "SceneComponent Object Reference"))
  (bind _ancestor (`local.Ancestor`))
  (set `local.Ancestor` (`SceneComponent.GetAttachParent` (`self.DefaultSceneRoot`)))
  (while (`KismetSystemLibrary.IsValid` _ancestor)
    (bind (_is_wanted_wire _wanted_wire) (`self.Is Wanted Wire` null _ancestor)
      (:`Yes`
        (return _wanted_wire))
      (:`No`
        (set `local.Ancestor` (`SceneComponent.GetAttachParent` (`local.Ancestor`))))))
  (return null))

(fn `Hide All Spline Meshes`
  (for _array_element (`self.Spline Meshes`)
    (`SceneComponent.SetVisibility` _array_element false false)))

(fn `NormalizeTangents`
  (for _index (range (+ (`SplineComponent.GetNumberOfSplinePoints` (`self.Spline`)) 1))
    (`SplineComponent.SetTangentsAtSplinePoint` (`self.Spline`) _index (* (`KismetMathLibrary.Normal` (`SplineComponent.GetArriveTangentAtSplinePoint` (`self.Spline`) _index "Local")) (`self.Normalized Tangent Length`)) (* (`KismetMathLibrary.Normal` (`SplineComponent.GetLeaveTangentAtSplinePoint` (`self.Spline`) _index "Local")) (`self.Normalized Tangent Length`)) "Local" true)))

(fn `Render`
  (`|ExecutionSequence`
    (:`then_0`
      ;[1 1 1] Read wire node positions.
      (set `self.Points` (`AGX_WireComponent.GetRenderNodeLocations` (`self.Wire`)))
      (if (`self.Debug Render Wire Points`)
        (`self.Debug Draw Wire`)))
    (:`then_1`
      ;[1 1 1] Call the selected rendering implementation.
      (switch `/AGXUnreal/Wire/EWireRenderMeshMode` (`self.Algorithm`)
        (:`NewEnumerator0`
          (`self.Render One Spline Mesh Per Wire Segment`))
        (:`NewEnumerator1`
          (`self.Render Fixed Segment Length`))))))

(fn `Render Fixed Segment Length`
  (bind _spline (`self.Spline`))
  (bind _num_spline_segments (`self.Num Spline Segments`))
  (bind _spline_2 (`self.Spline`))
  (bind _num_spline_segments_2 (`self.Num Spline Segments`))
  (bind _spline_3 (`self.Spline`))
  (bind _spline_4 (`self.Spline`))
  (bind _returnvalue (* (`AGX_WireComponent.Radius` (`self.Wire`)) 0.02))
  (bind _returnvalue_2 (`KismetMathLibrary.MakeVector2D` _returnvalue _returnvalue))
  (`|ExecutionSequence`
    (:`then_0`
      ;[1 1 1] Create Spline from Wire node locations.
      (`SplineComponent.ClearSplinePoints` _spline_3 false)
      (for _array_element (`self.Points`)
        (`SplineComponent.AddSplinePoint` _spline_3 _array_element "World" false))
      (switch `/AGXUnreal/Wire/EWireRenderTangentMode` (`self.Tangent Mode`)
        (:`NewEnumerator0`
          _)
        (:`NewEnumerator1`
          (`self.Distance Scale Tangents`))
        (:`NewEnumerator2`
          (`self.NormalizeTangents`)))
      (`SplineComponent.UpdateSpline` _spline_3)
      (if (`self.Debug Render Spline Tangents`)
        (for _index (range (+ (`SplineComponent.GetNumberOfSplinePoints` _spline_4) 1))
          (bind _returnvalue_3 (`SplineComponent.GetLocationAtSplinePoint` _spline_4 _index "World"))
          (`KismetSystemLibrary.DrawDebugLine` _returnvalue_3 (+ _returnvalue_3 (`SplineComponent.GetLeaveTangentAtSplinePoint` _spline_4 _index "World")) (struct :`R` 0.760417 :`A` 1.0) 0.0 1.0)
          (`KismetSystemLibrary.DrawDebugLine` _returnvalue_3 (- _returnvalue_3 (`SplineComponent.GetArriveTangentAtSplinePoint` _spline_4 _index "World")) (struct :`G` 0.097717 :`B` 0.71875 :`A` 1.0) 0.0 1.0))))
    (:`then_1`
      ;[1 1 1] Compute number of Spline Meshes to render.
      (set `self.Num Spline Segments` (`KismetMathLibrary.FCeil` (/ (`AGX_WireComponent.GetRestLength_BP` (`self.Wire`)) (`self.Segment Length`)))))
    (:`then_2`
      ;[1 1 1] Create missing Spline Meshes.
      (while (< (`KismetArrayLibrary.Array_Length` (`self.Spline Meshes`)) (`self.Num Spline Segments`))
        (`self.Create Spline Mesh`)))
    (:`then_3`
      ;[1 1 1] Set spline mesh visibility.
      (`|ExecutionSequence`
        (:`then_0`
          (for _index_2 (range _num_spline_segments_2)
            (`SceneComponent.SetVisibility` (`|GetArrayItem` (`self.Spline Meshes`) _index_2) true false)))
        (:`then_1`
          (for _index_3 (range _num_spline_segments_2 (+ (`KismetArrayLibrary.Array_LastIndex` (`self.Spline Meshes`)) 1))
            (`SceneComponent.SetVisibility` (`|GetArrayItem` (`self.Spline Meshes`) _index_3) false false)))))
    (:`then_4`
      ;[1 1 1] Position Spline Meshes at even distances along the Spline.
      (set `self.Current Segment Length` (/ (`SplineComponent.GetSplineLength` (`self.Spline`)) (`KismetMathLibrary.Conv_IntToDouble` (`self.Num Spline Segments`))))
      (for _index_4 (range (`self.Num Spline Segments`))
        (bind _output (`|GetArrayItem` (`self.Spline Meshes`) _index_4))
        (bind _returnvalue_4 (/ (`KismetMathLibrary.Conv_IntToDouble` _index_4) (`KismetMathLibrary.Conv_IntToDouble` _num_spline_segments)))
        (bind _returnvalue_5 (`SplineComponent.GetLocationAtTime` _spline_2 _returnvalue_4 "World" true))
        (bind _returnvalue_6 (/ (`KismetMathLibrary.Conv_IntToDouble` (+ _index_4 1)) (`KismetMathLibrary.Conv_IntToDouble` _num_spline_segments)))
        (bind _returnvalue_7 (`SplineComponent.GetLocationAtTime` _spline _returnvalue_6 "World" true))
        (`SplineMeshComponent.SetStartAndEnd` _output _returnvalue_5 (* (`KismetMathLibrary.Normal` (`SplineComponent.GetTangentAtTime` _spline_2 _returnvalue_4 "World" true)) (`self.Current Segment Length`)) _returnvalue_7 (* (`KismetMathLibrary.Normal` (`SplineComponent.GetTangentAtTime` _spline _returnvalue_6 "World" true)) (`self.Current Segment Length`)) false) ; These are in local space while the spline nodes has\nbeen positioned in world space. Not sure if and\nwhen that matters.
        (`SplineMeshComponent.SetStartScale` _output _returnvalue_2 false)
        (`SplineMeshComponent.SetEndScale` _output _returnvalue_2 false)
        (`SplineMeshComponent.UpdateMesh` _output)
        (if (`self.Debug Render Spline Mesh Points`)
          (`self.Debug Draw Spline Mesh` _returnvalue_5 _returnvalue_7))))))

(fn `Render One Spline Mesh Per Wire Segment`
  (bind _returnvalue (`KismetArrayLibrary.Array_LastIndex` (`self.Points`)))
  (`|ExecutionSequence`
    (:`then_0`
      ;[1 1 1] Create missing Spline Meshes.
      (while (> (- (`KismetArrayLibrary.Array_Length` (`self.Points`)) 1) (`KismetArrayLibrary.Array_Length` (`self.Spline Meshes`)))
        (`self.Create Spline Mesh`)))
    (:`then_1`
      ;[1 1 1] Set Spline Mesh visibility.
      (`|ExecutionSequence`
        (:`then_0`
          (for _index (range _returnvalue)
            (`SceneComponent.SetVisibility` (`|GetArrayItem` (`self.Spline Meshes`) _index) true false)))
        (:`then_1`
          (for _index_2 (range _returnvalue (+ (`KismetArrayLibrary.Array_LastIndex` (`self.Spline Meshes`)) 1))
            (`SceneComponent.SetVisibility` (`|GetArrayItem` (`self.Spline Meshes`) _index_2) false false)))))
    (:`then_2`
      (`self.ROSMPWS: Update All Meshes`))))

(fn `ROSMPWS: Update All Meshes`
  (bind _points (`self.Points`))
  (bind _points_2 (`self.Points`))
  (bind _points_3 (`self.Points`))
  (bind _returnvalue (`KismetArrayLibrary.Array_LastIndex` (`self.Points`)))
  (bind _returnvalue_2 (`KismetArrayLibrary.Array_Length` (`self.Points`)))
  (bind _output (`|GetArrayItem` (`self.Spline Meshes`)))
  (bind _output_2 (`|GetArrayItem` _points_3))
  (bind _output_3 (`|GetArrayItem` _points_3 1))
  (bind _output_4 (`|GetArrayItem` _points_2 _returnvalue))
  (`|ExecutionSequence`
    (:`then_0`
      ;[1 1 1] Update the first Spline Mesh.
      (if (>= _returnvalue_2 3)
        (`self.ROSMPWS: Update Mesh` _output _output_2 _output_2 _output_3 (`|GetArrayItem` _points_3 2))
        (elif (== _returnvalue_2 2)
          (`self.ROSMPWS: Update Mesh` _output _output_2 _output_2 _output_3 _output_3)
          (else
            (`KismetSystemLibrary.PrintString` "BP_WireRenderer got too few points.")))))
    (:`then_1`
      ;[1 1 1] Update internal Spline Meshes.
      (for _index (range 1 (+ (- (`KismetArrayLibrary.Array_LastIndex` (`self.Points`)) 2) 1))
        (`self.ROSMPWS: Update Mesh` (`|GetArrayItem` (`self.Spline Meshes`) _index) (`|GetArrayItem` _points (+ _index -1)) (`|GetArrayItem` _points _index) (`|GetArrayItem` _points (+ _index 1)) (`|GetArrayItem` _points (+ _index 2)))))
    (:`then_2`
      ;[1 1 1] Update the last Spline Mesh.
      (if (>= _returnvalue 2)
        (`self.ROSMPWS: Update Mesh` (`|GetArrayItem` (`self.Spline Meshes`) (- (`KismetArrayLibrary.Array_LastIndex` (`self.Points`)) 1)) (`|GetArrayItem` _points_2 (- _returnvalue 2)) (`|GetArrayItem` _points_2 (- _returnvalue 1)) _output_4 _output_4)))))

(fn `ROSMPWS: Update Mesh`
  (params (`Spline Mesh` :type "SplineMeshComponent Object Reference") (`Pn-1` :type "Vector Structure") (Pn :type "Vector Structure") (`Pn+1` :type "Vector Structure") (`Pn+2` :type "Vector Structure"))
  (bind _returnvalue (`KismetMathLibrary.Normal` (- (`local.Pn+2`) (`local.Pn`))))
  (bind _returnvalue_2 (`KismetMathLibrary.Normal` (- (`local.Pn+1`) (`local.Pn-1`))))
  (bind _returnvalue_3 (* (* (`AGX_WireComponent.Radius` (`self.Wire`)) (`self.Mesh Radius Scale`)) 0.02))
  ;[1 1 1] Can't this be done on construction only? Shouldn't change, I don't think.
  (`SplineMeshComponent.SetEndScale` `Spline Mesh` (`KismetMathLibrary.MakeVector2D` _returnvalue_3 _returnvalue_3) true)
  (`SplineMeshComponent.SetStartScale` `Spline Mesh` (`KismetMathLibrary.MakeVector2D` _returnvalue_3 _returnvalue_3) true)
  (`SplineMeshComponent.SetStartAndEnd` `Spline Mesh` (`local.Pn`) (select `bool` (`self.Normalize Tangents`) :`false` (* _returnvalue_2 (`KismetMathLibrary.VSize` (- (`local.Pn+1`) (`local.Pn`)))) :`true` _returnvalue_2) (`local.Pn+1`) (select `bool` (`self.Normalize Tangents`) :`false` (* _returnvalue (`KismetMathLibrary.VSize` (- (`local.Pn+1`) (`local.Pn`)))) :`true` _returnvalue) true)
  ;[1 1 1] Don't allow the wire segment direction to coninside with the Spline Up Dir, causes singularity that produces a zero-radius mesh.
  ; When close to vertical wire segment, set Spline Up Dir horizontal.
  ; Not sure what  that will do at the transition from a horizontal segment to a vertical one.
  (`SplineMeshComponent.SetSplineUpDir` `Spline Mesh` (`KismetMathLibrary.SelectVector` (`KismetMathLibrary.Vector_Forward`) (`KismetMathLibrary.Vector_Up`) (> (`KismetMathLibrary.Abs` (`KismetMathLibrary.Dot_VectorVector` (`KismetMathLibrary.Normal` (- (`local.Pn+1`) (`local.Pn`))) (`KismetMathLibrary.Vector_Up`))) 0.8)) true)
  (if (`self.Debug Render Spline Mesh Points`)
    (`self.Debug Draw Spline Mesh` (`local.Pn`) (`local.Pn+1`))))

(fn `Update Wire Reference`
  (params (`Suppress Warnings` :type Boolean))
  (returns (`Have Wire` :type Boolean))
  (bind _wiresoftref (`self.WireSoftRef`))
  ;[1 1 1] Determine if the Wire we want to render has been destroyed by a Blueprint Reconstruction or otherwise been removed. If so, try to find a new wire.
  (if (`KismetSystemLibrary.IsValidSoftObjectReference` _wiresoftref)
    (set `self.Wire` (`|ConvertAsset` _wiresoftref))
    (else
      (set `self.Wire` null)
      (`self.Find Wire` `Suppress Warnings`)))
  (return (`KismetSystemLibrary.IsValid` (`self.Wire`))))

(fn `UserConstructionScript`
  (bind _wire (`self.Wire`))
  ;[1 1 1] Deprecation message
  (`KismetSystemLibrary.PrintString` "BP_WireRenderer has been deprecated. AGX Wires now render themselves. Instances of BP_WireRenderer in the level should be removed. If you still wish to use the old BP_WireRenderer, copy it into your project, remove this deprecation message in it's construction script and then set Visible \"false\" on the AGX Wire." true true (struct :`G` 0.66 :`B` 1.0 :`A` 1.0) 20.0)
  ;[1 1 1] Remove the default spline points so the Spline isn't visible in the Viewport.
  ;;[1 1 1 1 12] The spline is an internal thing and should not be interacted with by the user. Is there a way to hide it completely?
  (`SplineComponent.ClearSplinePoints` (`self.Spline`) true)
  (`/Engine/EditorBlueprintResources/StandardMacros.IsValid` _wire
    (:`Is Valid`
      (set `self.WireSoftRef` (`|ConvertAsset` _wire))
      ;[1 1 1] Try to make a first render immediately. This is required when editing rendering settings during a paused Play In Editor session since Blueprint Reconstruction will destroy all Spline Meshes and they won't otherwise be created again until the next tick.
      (`self.Render` :!label _label))
    (:`Is Not Valid`
      (bind _have_wire (`self.Update Wire Reference` true))
      (if _have_wire
        (goto _label)))))