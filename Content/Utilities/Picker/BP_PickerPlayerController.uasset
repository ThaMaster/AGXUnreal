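; BP_PickerPlayerController is a player controller that drives a Picker component for grabbing things with the mouse.
; Left Shift sets a held flag, and pressing the left mouse button while it is held starts a long-reach grab for the first player.
; Releasing the mouse button ends the grab if the Picker is active, regardless of whether Shift is still held.
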(event `Key|LeftShift`
  (params (Key :type "Key Structure"))
  (:`Pressed`
    (set `self.bShiftDown` true))
  (:`Released`
    (set `self.bShiftDown` false)))

(event `Key|LeftMouseButton`
  (params (Key :type "Key Structure"))
  (:`Pressed`
    (if (`self.bShiftDown`)
      (`/AGXUnreal/Utilities/Picker/BP_Picker.Begin Grab` (`self.Picker`) 0 5000.0)))
  (:`Released`
    (if (`/AGXUnreal/Utilities/Picker/BP_Picker.Is Active` (`self.Picker`))
      (`/AGXUnreal/Utilities/Picker/BP_Picker.End Grab` (`self.Picker`)))))

(fn `UserConstructionScript`)