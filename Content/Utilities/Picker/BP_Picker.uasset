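; Picker utility that lets a player grab or pinch AGX rigid bodies from the camera view or mouse cursor.
; Begin functions clear any active constraint, line trace, then search the hit component's parents for an AGX rigid body.
; A found body gets a spawned camera or cursor lock actor, with separate grab and pinch rotation elasticity and damping.
; That single active constraint actor defines the interaction state and is destroyed on end.
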(fn `Begin Camera Grab`
  (params (`Player Index` :type Integer) (`Reach Length` :type "Float (double-precision)"))
  (bind _returnvalue (`GameplayStatics.GetPlayerPawn` `Player Index`))
  (`self.Destroy Any Active Constraint`)
  (bind (_body _body_transform_no_scale _anchor_to_body) (`self.Line Trace for Body from Camera` `Player Index` `Reach Length` _returnvalue))
  (`self.Spawn Camera Grab Constraint` _body _body_transform_no_scale _anchor_to_body _returnvalue))

(fn `Begin Camera Pinch`
  (params (`Player Index` :type Integer) (`Reach Length` :type "Float (double-precision)"))
  (bind _returnvalue (`GameplayStatics.GetPlayerPawn` `Player Index`))
  (`self.Destroy Any Active Constraint`)
  (bind (_body _body_transform_no_scale _anchor_to_body _hit_location _anchor_to_hit_location) (`self.Line Trace for Body from Camera` `Player Index` `Reach Length` _returnvalue))
  (`self.Spawn Camera Pinch Constraint` _body _hit_location _anchor_to_hit_location _returnvalue))

(fn `Begin Cursor Grab`
  (params (`Player Index` :type Integer) (`Reach Length` :type "Float (double-precision)"))
  (`self.Destroy Any Active Constraint`)
  (bind (_body _body_transform_no_scale _anchor_to_body _hit_location _anchor_to_hit_location _distance) (`self.Line Trace for Body from Cursor` `Player Index` `Reach Length` (`GameplayStatics.GetPlayerPawn` `Player Index`)))
  (`self.Spawn Cursor Grab Constraint` _body _hit_location _distance))

(fn `Begin Cursor Pinch`
  (params (`Player Index` :type Integer) (Reach :type "Float (double-precision)"))
  (`self.Destroy Any Active Constraint`)
  (bind (_body _body_transform_no_scale _anchor_to_body _hit_location _anchor_to_hit_location _distance) (`self.Line Trace for Body from Cursor` `Player Index` Reach (`GameplayStatics.GetPlayerPawn` `Player Index`)))
  (`self.Spawn Cursor Pinch Constraint` _body _hit_location _distance))

(fn `Destroy Any Active Constraint`
  (bind _active_constraint (`self.Active Constraint`))
  (`/Engine/EditorBlueprintResources/StandardMacros.IsValid` _active_constraint
    (:`Is Valid`
      (`Actor.K2_DestroyActor` _active_constraint))
    (:`Is Not Valid`
      _))
  (return))

(fn `End Interaction`
  (bind _active_constraint (`self.Active Constraint`))
  (`/Engine/EditorBlueprintResources/StandardMacros.IsValid` _active_constraint
    (:`Is Valid`
      (`Actor.K2_DestroyActor` _active_constraint))))

(fn `Is Interacting`
  (returns (bIsPicking :type Boolean))
  (return (`KismetSystemLibrary.IsValid` (`self.Active Constraint`))))

(fn `Line Trace for Body`
  (params (Start :type "Vector Structure") (End :type "Vector Structure") (Anchor :type "Actor Object Reference"))
  (returns (Body :type "AGX_RigidBodyComponent Object Reference") (`Body Transform No Scale` :type "Transform Structure") (`Anchor To Body` :type "Vector Structure") (`Hit Location` :type "Vector Structure") (`Anchor To Hit Location` :type "Vector Structure") (Distance :type "Float (double-precision)"))
  (locals (`Return Body` :type "AGX_RigidBodyComponent Object Reference") (`Return Body Transform No Scale` :type "Transform Structure") (`Return Anchor to Body` :type "Vector Structure" :default (0.0 0.0 0.0)) (`Return Hit Location` :type "Vector Structure") (`Return Actor To Hit Location` :type "Vector Structure" :default (0.0 0.0 0.0)) (`Return Distance` :type "Float (double-precision)" :default 0.0))
  (bind _returnvalue (`Actor.GetTransform` Anchor))
  (bind (_outhit _returnvalue_2) (`KismetSystemLibrary.LineTraceSingle` :`Start` Start :`End` End :`TraceChannel` "TraceTypeQuery1" :`bTraceComplex` true :`DrawDebugType` "ForDuration"))
  (if _returnvalue_2
    (for _array_element (`SceneComponent.GetParentComponents` (`.HitComponent` (`GameplayStatics.BreakHitResult` _outhit)))
      (bind _asagx_rigid_body_component (cast `AGX_RigidBodyComponent` _array_element))
      (set `local.Return Body` _asagx_rigid_body_component)
      (bind _returnvalue_3 (`SceneComponent.K2_GetComponentLocation` _asagx_rigid_body_component))
      (set `local.Return Body Transform No Scale` (`KismetMathLibrary.MakeTransform` _returnvalue_3 (`SceneComponent.K2_GetComponentRotation` _asagx_rigid_body_component)))
      (set `local.Return Distance` (`.Distance` (`GameplayStatics.BreakHitResult` _outhit)))
      (set `local.Return Hit Location` (`.Location` (`GameplayStatics.BreakHitResult` _outhit)))
      (set `local.Return Anchor to Body` (`KismetMathLibrary.InverseTransformLocation` _returnvalue _returnvalue_3))
      (set `local.Return Actor To Hit Location` (`KismetMathLibrary.InverseTransformLocation` _returnvalue (`.Location` (`GameplayStatics.BreakHitResult` _outhit))))
      (break))
    (return (`local.Return Body`) (`local.Return Body Transform No Scale`) (`local.Return Anchor to Body`) (`local.Return Hit Location`) (`local.Return Actor To Hit Location`) (`local.Return Distance`))))

(fn `Line Trace for Body from Camera`
  (params (PlayerIndex :type Integer) (Reach :type "Float (double-precision)") (Anchor :type "Actor Object Reference"))
  (returns (Body :type "AGX_RigidBodyComponent Object Reference") (`Body Transform No Scale` :type "Transform Structure") (`Anchor to Body` :type "Vector Structure") (`Hit Location` :type "Vector Structure") (`Anchor to Hit Location` :type "Vector Structure"))
  (bind _returnvalue (`GameplayStatics.GetPlayerCameraManager` PlayerIndex))
  (bind _returnvalue_2 (`PlayerCameraManager.GetCameraLocation` _returnvalue))
  (bind (_body _body_transform_no_scale _anchor_to_body _hit_location _anchor_to_hit_location) (`self.Line Trace for Body` _returnvalue_2 (+ _returnvalue_2 (* (`KismetMathLibrary.GetForwardVector` (`PlayerCameraManager.GetCameraRotation` _returnvalue)) Reach)) Anchor))
  (return _body _body_transform_no_scale _anchor_to_body _hit_location _anchor_to_hit_location))

(fn `Line Trace for Body from Cursor`
  (params (`Player Index` :type Integer) (Reach :type "Float (double-precision)") (Anchor :type "Actor Object Reference"))
  (returns (Body :type "AGX_RigidBodyComponent Object Reference") (`Body Transform No Scale` :type "Transform Structure") (`Anchor to Body` :type "Vector Structure") (`Hit Location` :type "Vector Structure") (`Anchor to Hit Location` :type "Vector Structure") (Distance :type "Float (double-precision)"))
  (bind (_worldlocation _worlddirection) (`PlayerController.DeprojectMousePositionToWorld` (`GameplayStatics.GetPlayerController` `Player Index`)))
  (bind (_body _body_transform_no_scale _anchor_to_body _hit_location _anchor_to_hit_location _distance) (`self.Line Trace for Body` _worldlocation (+ _worldlocation (* _worlddirection Reach)) Anchor))
  (return _body _body_transform_no_scale _anchor_to_body _hit_location _anchor_to_hit_location _distance))

(fn `Spawn Camera Grab Constraint`
  (params (Body :type "AGX_RigidBodyComponent Object Reference") (`Body Transform No Scale` :type "Transform Structure") (`Anchor to Body` :type "Vector Structure") (Anchor :type "Actor Object Reference"))
  (`/Engine/EditorBlueprintResources/StandardMacros.IsValid` Body
    (:`Is Valid`
      (bind _returnvalue (`|SpawnActorFromClass` "/AGXUnreal/Utilities/Picker/BP_PickerCameraLock.BP_PickerCameraLock_C" `Body Transform No Scale` "Undefined" "OverrideRootScale" null Anchor `Anchor to Body` Body (`self.Grab Elasticity`) (`self.Grab Damping`) null))
      (set `self.Active Constraint` _returnvalue))))

(fn `Spawn Camera Pinch Constraint`
  (params (Body :type "AGX_RigidBodyComponent Object Reference") (`Hit Location` :type "Vector Structure") (`Anchor to Hit Location` :type "Vector Structure") (Anchor :type "Actor Object Reference"))
  (`/Engine/EditorBlueprintResources/StandardMacros.IsValid` Body
    (:`Is Valid`
      (bind _returnvalue (`|SpawnActorFromClass` "/AGXUnreal/Utilities/Picker/BP_PickerCameraLock.BP_PickerCameraLock_C" (`KismetMathLibrary.Conv_VectorToTransform` `Hit Location`) "Undefined" "OverrideRootScale" null Anchor `Anchor to Hit Location` Body (`self.Pinch Elasticity`) (`self.Pinch Damping`) null))
      (set `self.Active Constraint` _returnvalue))))

(fn `Spawn Cursor Grab Constraint`
  (params (Body :type "AGX_RigidBodyComponent Object Reference") (`Hit Location` :type "Vector Structure") (Distance :type "Float (double-precision)"))
  (`/Engine/EditorBlueprintResources/StandardMacros.IsValid` Body
    (:`Is Valid`
      (bind _returnvalue (`|SpawnActorFromClass` "/AGXUnreal/Utilities/Picker/BP_PickerCursorLock.BP_PickerCursorLock_C" (`KismetMathLibrary.Conv_VectorToTransform` `Hit Location`) "Undefined" "OverrideRootScale" null Distance Body (`self.Grab Elasticity`) (`self.Grab Damping`) null))
      (set `self.Active Constraint` _returnvalue))))

(fn `Spawn Cursor Pinch Constraint`
  (params (Body :type "AGX_RigidBodyComponent Object Reference") (`Hit Location` :type "Vector Structure") (Distance :type "Float (double-precision)"))
  (`/Engine/EditorBlueprintResources/StandardMacros.IsValid` Body
    (:`Is Valid`
      (bind _returnvalue (`|SpawnActorFromClass` "/AGXUnreal/Utilities/Picker/BP_PickerCursorLock.BP_PickerCursorLock_C" (`KismetMathLibrary.Conv_VectorToTransform` `Hit Location`) "Undefined" "OverrideRootScale" null Distance Body (`self.Pinch Elasticity`) (`self.Pinch Damping`) null))
      (set `self.Active Constraint` _returnvalue))))