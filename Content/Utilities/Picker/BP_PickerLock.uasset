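; BP_PickerLock is a picker utility that constrains a body to a point that follows an anchor actor.
; On construction, it assigns a valid Body to its constraint component and applies a shared rotation elasticity to all three rotational axes.
; Each tick, it transforms an attachment offset by the Anchor's transform and sets it as the constraint's second attachment location.
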(event `self.ReceiveTick`
  (params (DeltaSeconds :type "Float (single-precision)"))
  (`AGX_ConstraintComponent.SetConstraintAttachmentLocation2` (`self.ConstraintComponent`) (`KismetMathLibrary.TransformLocation` (`self.GetTransform` (`self.Anchor`)) (`self.ToAttachment`))))

(fn `UserConstructionScript`
  (bind _body (`self.Body`))
  (bind _constraintcomponent (`self.ConstraintComponent`))
  (bind _rotation_elasticity (`self.Rotation Elasticity`))
  (if (`KismetSystemLibrary.IsValid` _body)
    (`AGX_ConstraintComponent.SetBody1` (`self.ConstraintComponent`) _body)
    (`AGX_ConstraintComponent.SetElasticity` _constraintcomponent "Rotational1" _rotation_elasticity)
    (`AGX_ConstraintComponent.SetElasticity` _constraintcomponent "Rotational2" _rotation_elasticity)
    (`AGX_ConstraintComponent.SetElasticity` _constraintcomponent "Rotational3" _rotation_elasticity)))